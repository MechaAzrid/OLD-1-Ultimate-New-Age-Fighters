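; Test 2D Naruto flipbook character combining player-style input (walk, double-tap run, double jump, defend/roll, three-step attack) with simple chase AI.
; Input events set CharacterState and walk speed, while Tick resolves facing and movement state and calls Set*State functions to swap directional flipbooks.
; Double-tap detection chains AxisSplit, DoOnce edge triggers and a timed DoN.
; PawnSensing moves it toward seen Paper2D_Characters and alters the player's FullHealth on arrival.
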(event OnSeePawn(PawnSensing)
  (params (Pawn :type Pawn%20Object%20Reference))
  (bind _aspaper_2d_character (Utilities|Casting|CastToPaper2D_Character Pawn))
  (AI|AIMoveTo self "0, 0, 0" _aspaper_2d_character 5.0 false
    (:then
      (Transformation|SetWorldRotation (Variables|Default|GetSprite) (Math|Rotator|MakeRotator 0.0 0.0 -9e+01) false false))
    (:OnSuccess
      (bind _aspaper_2d_character_2 (Utilities|Casting|CastToPaper2D_Character (Game|GetPlayerCharacter 0)))
      (Variables|/Game/Blueprints/Paper2D_Character.Paper2D_Character_C|SetfullHealth _aspaper_2d_character_2 (- (Variables|Default|GetfullHealth) 5e+02)))))

(event Custom|DirectionAndMovementStates
  ;[1 1 1] Set Direction and Movements States
  (if (Utilities|IsFalling)
    ;;[1 1 1] If Character Is Jumping, (Even Though Character Is Falling), Don't Play Fall Anim Until Playing Is No Longer Jumping
    (if (not (Utilities|Enum|Equal(Enum) (Variables|Default|GetCharacterState) "NewEnumerator3"))
      (Variables|Default|SetCharacterState "NewEnumerator4")
      (CallFunction|SetFallingState))
    (else
      (if (and (> (Variables|/Script/Engine.CharacterMovementComponent|GetMaxWalkSpeed (Variables|Character|GetCharacterMovement)) 6.5e+02) (not (Utilities|IsVelocityZero)))
        (Variables|Default|SetCharacterState "NewEnumerator1")
        (elif (and (> (Variables|/Script/Engine.CharacterMovementComponent|GetMaxWalkSpeed (Variables|Character|GetCharacterMovement)) 3.5e+02) (not (Utilities|IsVelocityZero)))
          (Variables|Default|SetCharacterState "NewEnumerator14")))
      (if (or (!= (Input|AxisValues|GetXAxis) 0.0) (!= (Input|AxisValues|GetYAxis) 0.0))
        (CallFunction|SetDirection :!label _label)
        (if (Utilities|Enum|Equal(Enum) (Variables|Default|GetCharacterState) "NewEnumerator0")
          (CallFunction|SetWalkingState)
          (Utilities|FlowControl|Delay 0.47)
          (Audio|PlaySound2D "/Game/Audio/Sound_Effects/Running.Running" 1.0 1.0 0.0 0 0)
          (elif (Utilities|Enum|Equal(Enum) (Variables|Default|GetCharacterState) "NewEnumerator1")
            (CallFunction|SetRunningState)
            (Utilities|FlowControl|Delay 0.3)
            (Audio|PlaySound2D "/Game/Audio/Sound_Effects/Running.Running" 1.0 1.0 0.0 0 0)))
        (else
          (Utilities|FlowControl|Delay 0.15)
          (if (or (!= (Input|AxisValues|GetXAxis) 0.0) (!= (Input|AxisValues|GetYAxis) 0.0))
            (goto _label)
            (else
              ;;[1 1 1] Check If Player Is Defending = If Not True Return To Idle
              (if (Utilities|Enum|Equal(Enum) (Variables|Default|GetCharacterState) "NewEnumerator8")
                (CallFunction|SetDefendState)
                (elif (Utilities|Enum|Equal(Enum) (Variables|Default|GetCharacterState) "NewEnumerator7")
                  (CallFunction|SetAttackState)
                  (elif (Utilities|Enum|Equal(Enum) (Variables|Default|GetCharacterState) "NewEnumerator12")
                    (CallFunction|SetGetHurtState)
                    (elif (Utilities|Enum|Equal(Enum) (Variables|Default|GetCharacterState) "NewEnumerator14")
                      (CallFunction|SetDashing/RollingState)
                      (elif (not (Utilities|IsFalling))
                        (CallFunction|SetIdleState)))))))))))))

(event EventTick
  (params (DeltaSeconds :type Float%20%28single-precision%29))
  ;[1 1 1] Player Direction
  (CallFunction|DirectionandMovementStates))

(event EventOnLanded
  (params (Hit :type Hit%20Result%20Structure%20%28by%20ref%29))
  ;[1 1 1] Jumping/Double Jumping
  (Audio|PlaySound2D "/Game/Audio/Sound_Effects/Landing.Landing" 1.0 1.0 0.0 0 0)
  (Variables|Default|SetCharacterState "NewEnumerator9")
  (CallFunction|SetCrouchLandState)
  (Utilities|FlowControl|DoN 2) ; enters at Reset
)

(event Input|ActionEvents|InputActionDefending
  (params (Key :type Key%20Structure))
  (:Pressed
    (if (Utilities|Enum|Equal(Enum) (Variables|Default|GetCharacterState) "NewEnumerator1")
      (Variables|Default|SetCharacterState "NewEnumerator14")
      (CallFunction|SetDashing/RollingState)
      (Variables|/Script/Engine.CharacterMovementComponent|SetMaxWalkSpeed (Variables|Character|GetCharacterMovement) 4e+02)
      (else
        (Variables|Default|SetCharacterState "NewEnumerator8")
        (CallFunction|SetDefendState)
        (Variables|/Script/Engine.CharacterMovementComponent|SetMaxWalkSpeed (Variables|Character|GetCharacterMovement) 1.5e+02))))
  (:Released
    (Variables|Default|SetCharacterState "NewEnumerator6")
    (CallFunction|SetIdleState)))

(event Input|ActionEvents|InputActionJumping
  (params (Key :type Key%20Structure))
  ;[1 1 1] Jumping/Double Jumping
  (:Pressed
    (bind _counter (Utilities|FlowControl|DoN 2)
      (:Exit
        (switch int _counter
          (:1
            (Variables|Default|SetCharacterState "NewEnumerator9")
            (CallFunction|SetCrouchLandState)
            (Variables|Default|SetCharacterState "NewEnumerator11")
            (CallFunction|SetCrouchJumpState)
            (Character|Jump)
            (Audio|PlaySound2D "/Game/Audio/Sound_Effects/Naruto_Jump_SFX.Naruto_Jump_SFX" 1.0 1.0 0.0 0 0)
            (Variables|Default|SetCharacterState "NewEnumerator3")
            (CallFunction|SetJumpingState))
          (:2
            (Character|LaunchCharacter "0,0.000000,600.000000" false true)
            (Audio|PlaySound2D "/Game/Audio/Sound_Effects/Naruto_Jump_SFX.Naruto_Jump_SFX" 1.0 1.0 0.0 0 0)
            (Variables|Default|SetCharacterState "NewEnumerator3")
            (CallFunction|SetJumpingState))))))
  (:Released
    (Character|StopJumping)
    (Variables|Default|SetCharacterState "NewEnumerator4")
    (CallFunction|SetFallingState)))

(event Input|ActionEvents|InputActionAttacking
  (params (Key :type Key%20Structure))
  ;[1 1 1] Attacking
  (:Pressed
    (bind _counter (Utilities|FlowControl|DoN 3)
      (:Exit
        (switch int _counter
          (:1
            (Variables|Default|SetCharacterState "NewEnumerator7")
            (CallFunction|SetLightAttackState))
          (:2
            (Variables|Default|SetCharacterState "NewEnumerator7")
            (CallFunction|SetMediumAttackState))
          (:3
            (Variables|Default|SetCharacterState "NewEnumerator7")
            (CallFunction|SetHeavyAttackState)))))))

(event Input|AxisEvents|InputAxisXAxis
  (params (AxisValue :type Float%20%28single-precision%29))
  ;[1 1 1] Axis Movement (Up, Down | Left, Right = Walking) || Double Tap Axis Movement (Up, Down | Left, Right = Running)
  (if (not (Utilities|Enum|Equal(Enum) (Variables|Default|GetCharacterState) "NewEnumerator8"))
    (Utilities|FlowControl|Sequence
      (:then_0
        (if (Math|Boolean|ORBoolean (Utilities|IsFalling) (Utilities|Enum|Equal(Enum) (Variables|Default|GetCharacterState) "NewEnumerator1") (Utilities|Enum|Equal(Enum) (Variables|Default|GetCharacterState) "NewEnumerator3") (Utilities|IsVelocityZero))
          _
          (else
            (Variables|Default|SetCharacterState "NewEnumerator0")))
        (Pawn|Input|AddMovementInput "0,1.000000, 0" AxisValue false))
      (:then_1
        (if (Math|Boolean|ORBoolean (Utilities|IsVelocityGreaterThanZero) (Utilities|Enum|Equal(Enum) (Variables|Default|GetCharacterState) "NewEnumerator8") (Utilities|Enum|Equal(Enum) (Variables|Default|GetCharacterState) "NewEnumerator3") (Utilities|Enum|Equal(Enum) (Variables|Default|GetCharacterState) "NewEnumerator7"))
          (Utilities|AxisDoubleTap AxisValue (Variables|Default|GetaxisThreshold) (Variables|Default|GetTimeout)
            (:Positive
              _)
            (:Negative
              _))
          ;;[1 1 1] Running
          (Variables|Default|SetCharacterState "NewEnumerator1")
          (Variables|/Script/Engine.CharacterMovementComponent|SetMaxWalkSpeed (Variables|Character|GetCharacterMovement) 7.5e+02)
          (else
            (if (Utilities|IsVelocityGreaterThanZero)
              (Variables|Default|SetCharacterState "NewEnumerator0")
              (else
                (Variables|Default|SetCharacterState "NewEnumerator6")))
            (Variables|/Script/Engine.CharacterMovementComponent|SetMaxWalkSpeed (Variables|Character|GetCharacterMovement) 1.5e+02)))))))

(event Input|AxisEvents|InputAxisYAxis
  (params (AxisValue :type Float%20%28single-precision%29))
  ;[1 1 1] Axis Movement (Up, Down | Left, Right = Walking) || Double Tap Axis Movement (Up, Down | Left, Right = Running)
  (if (not (Utilities|Enum|Equal(Enum) (Variables|Default|GetCharacterState) "NewEnumerator8"))
    (Utilities|FlowControl|Sequence
      (:then_0
        (if (Math|Boolean|ORBoolean (Utilities|IsFalling) (Utilities|Enum|Equal(Enum) (Variables|Default|GetCharacterState) "NewEnumerator1") (Utilities|Enum|Equal(Enum) (Variables|Default|GetCharacterState) "NewEnumerator3") (Utilities|IsVelocityZero))
          _
          (else
            (Variables|Default|SetCharacterState "NewEnumerator0")))
        (Pawn|Input|AddMovementInput "-1.000000,0.000000, 0" AxisValue false))
      (:then_1
        (if (Math|Boolean|ORBoolean (Utilities|IsVelocityGreaterThanZero) (Utilities|Enum|Equal(Enum) (Variables|Default|GetCharacterState) "NewEnumerator8") (Utilities|Enum|Equal(Enum) (Variables|Default|GetCharacterState) "NewEnumerator3") (Utilities|Enum|Equal(Enum) (Variables|Default|GetCharacterState) "NewEnumerator7"))
          (Utilities|AxisDoubleTap AxisValue (Variables|Default|GetaxisThreshold) (Variables|Default|GetTimeout)
            (:Positive
              _)
            (:Negative
              _))
          ;;[1 1 1] Running
          (Variables|Default|SetCharacterState "NewEnumerator1")
          (Variables|/Script/Engine.CharacterMovementComponent|SetMaxWalkSpeed (Variables|Character|GetCharacterMovement) 7.5e+02)
          (else
            (if (Utilities|IsVelocityGreaterThanZero)
              (Variables|Default|SetCharacterState "NewEnumerator0")
              (else
                (Variables|Default|SetCharacterState "NewEnumerator6")))
            (Variables|/Script/Engine.CharacterMovementComponent|SetMaxWalkSpeed (Variables|Character|GetCharacterMovement) 1.5e+02)))))))

(fn ConstructionScript
  ;[1 1 1] World Rotation
)

(fn SetDirectionOld
  (if (or (!= (Input|AxisValues|GetXAxis) 0.0) (!= (Input|AxisValues|GetYAxis) 0.0))
    (bind _output_get (Variables|Default|SetDirection (select (> (Input|AxisValues|GetYAxis) 0.0) "NewEnumerator0" (select (< (Input|AxisValues|GetYAxis) 0.0) "NewEnumerator1" (select (> (Input|AxisValues|GetXAxis) 0.0) "NewEnumerator2" "NewEnumerator3")))))
    (switch Utilities|FlowControl|Switch|SwitchonSetDir _output_get
      (:NewEnumerator0
        _)
      (:NewEnumerator1
        _)
      (:NewEnumerator2
        (Variables|Default|SetisFacingLeft true)
        (Variables|Default|SetisFacingRight false))
      (:NewEnumerator3
        (Variables|Default|SetisFacingRight true)
        (Variables|Default|SetisFacingLeft false)))
    (return)))

(fn CalculateZ
  (bind _returnvalue (Transformation|GetActorLocation))
  (bind _returnvalue_2 (Transformation|GetActorLocation))
  (bind _outhit (Collision|LineTraceByChannel (Transformation|GetActorLocation) (Math|Vector|MakeVector (.x _returnvalue_2) (.y _returnvalue_2) (- (.z _returnvalue_2) 2e+02)) "TraceTypeQuery1" false 0 "None"))
  (Transformation|SetActorLocation (Math|Vector|MakeVector (.x _returnvalue) (.y _returnvalue) (+ (.z (.ImpactPoint (Collision|BreakHitResult _outhit))) (Variables|Default|GetDistanceZ))) false false))

(fn SetIdleState
  (bind _direction (Variables|Default|GetDirection))
  (Variables|Default|SetCharacterState "NewEnumerator6")
  (Sprite|SetFlipbook (Variables|Default|GetSprite) (select (Utilities|IsVelocityGreaterThanZero) 0 (select (Variables|Default|GetisFacingRight) (Utilities|Select :Index _direction :NewEnumerator0 "/Game/Animations/Characters/Templates/New_Naruto/New_Naruto_Idle_FR.New_Naruto_Idle_FR" :NewEnumerator1 "/Game/Animations/Characters/Templates/New_Naruto/New_Naruto_Idle_FR.New_Naruto_Idle_FR" :NewEnumerator2 "/Game/Animations/Characters/Templates/New_Naruto/New_Naruto_Idle_FR.New_Naruto_Idle_FR" :NewEnumerator3 "/Game/Animations/Characters/Templates/New_Naruto/New_Naruto_Idle_FR.New_Naruto_Idle_FR") (Utilities|Select :Index _direction :NewEnumerator0 "/Game/Animations/Characters/Templates/New_Naruto/New_Naruto_Idle_FL.New_Naruto_Idle_FL" :NewEnumerator1 "/Game/Animations/Characters/Templates/New_Naruto/New_Naruto_Idle_FL.New_Naruto_Idle_FL" :NewEnumerator2 "/Game/Animations/Characters/Templates/New_Naruto/New_Naruto_Idle_FL.New_Naruto_Idle_FL" :NewEnumerator3 "/Game/Animations/Characters/Templates/New_Naruto/New_Naruto_Idle_FL.New_Naruto_Idle_FL")))))

(fn SetDirection
  (bind _output_get (Variables|Default|SetDirection (select (> (Input|AxisValues|GetYAxis) 0.0) "NewEnumerator0" (select (< (Input|AxisValues|GetYAxis) 0.0) "NewEnumerator1" (select (> (Input|AxisValues|GetXAxis) 0.0) "NewEnumerator2" "NewEnumerator3")))))
  (switch Utilities|FlowControl|Switch|SwitchonSetDir _output_get
    (:NewEnumerator0
      _)
    (:NewEnumerator1
      _)
    (:NewEnumerator2
      (Variables|Default|SetisFacingLeft true)
      (Variables|Default|SetisFacingRight false))
    (:NewEnumerator3
      (Variables|Default|SetisFacingRight true)
      (Variables|Default|SetisFacingLeft false)))
  (return))

(fn SetWalkingState
  (bind _direction (Variables|Default|GetDirection))
  (Sprite|SetFlipbook (Variables|Default|GetSprite) (select (Variables|Default|GetisFacingRight) (Utilities|Select :Index _direction :NewEnumerator0 "/Game/Animations/Characters/Templates/New_Naruto/New_Naruto_Walk_FR.New_Naruto_Walk_FR" :NewEnumerator1 "/Game/Animations/Characters/Templates/New_Naruto/New_Naruto_Walk_FR.New_Naruto_Walk_FR" :NewEnumerator2 "/Game/Animations/Characters/Templates/New_Naruto/New_Naruto_Walk_FR.New_Naruto_Walk_FR" :NewEnumerator3 "/Game/Animations/Characters/Templates/New_Naruto/New_Naruto_Walk_FR.New_Naruto_Walk_FR") (Utilities|Select :Index _direction :NewEnumerator0 "/Game/Animations/Characters/Templates/New_Naruto/New_Naruto_Walk_FL.New_Naruto_Walk_FL" :NewEnumerator1 "/Game/Animations/Characters/Templates/New_Naruto/New_Naruto_Walk_FL.New_Naruto_Walk_FL" :NewEnumerator2 "/Game/Animations/Characters/Templates/New_Naruto/New_Naruto_Walk_FL.New_Naruto_Walk_FL" :NewEnumerator3 "/Game/Animations/Characters/Templates/New_Naruto/New_Naruto_Walk_FL.New_Naruto_Walk_FL"))))

(fn SetRunningState
  (Sprite|SetFlipbook (Variables|Default|GetSprite) (select (Variables|Default|GetisFacingRight) (Utilities|Select :Index (Variables|Default|GetDirection) :NewEnumerator0 "/Game/Animations/Characters/Templates/New_Naruto/New_Naruto_Run_FR.New_Naruto_Run_FR" :NewEnumerator1 "/Game/Animations/Characters/Templates/New_Naruto/New_Naruto_Run_FR.New_Naruto_Run_FR" :NewEnumerator2 "/Game/Animations/Characters/Templates/New_Naruto/New_Naruto_Run_FR.New_Naruto_Run_FR" :NewEnumerator3 "/Game/Animations/Characters/Templates/New_Naruto/New_Naruto_Run_FR.New_Naruto_Run_FR") (Utilities|Select :Index (Variables|Default|GetDirection) :NewEnumerator0 "/Game/Animations/Characters/Templates/New_Naruto/New_Naruto_Run_FL.New_Naruto_Run_FL" :NewEnumerator1 "/Game/Animations/Characters/Templates/New_Naruto/New_Naruto_Run_FL.New_Naruto_Run_FL" :NewEnumerator2 "/Game/Animations/Characters/Templates/New_Naruto/New_Naruto_Run_FL.New_Naruto_Run_FL" :NewEnumerator3 "/Game/Animations/Characters/Templates/New_Naruto/New_Naruto_Run_FL.New_Naruto_Run_FL"))))

(fn SetJumpingState
  (bind _direction (Variables|Default|GetDirection))
  (Sprite|SetFlipbook (Variables|Default|GetSprite) (select (Variables|Default|GetisFacingRight) (Utilities|Select :Index _direction :NewEnumerator0 "/Game/Animations/Characters/Templates/New_Naruto/New_Naruto_Jump_FR.New_Naruto_Jump_FR" :NewEnumerator1 "/Game/Animations/Characters/Templates/New_Naruto/New_Naruto_Jump_FR.New_Naruto_Jump_FR" :NewEnumerator2 "/Game/Animations/Characters/Templates/New_Naruto/New_Naruto_Jump_FR.New_Naruto_Jump_FR" :NewEnumerator3 "/Game/Animations/Characters/Templates/New_Naruto/New_Naruto_Jump_FR.New_Naruto_Jump_FR") (Utilities|Select :Index _direction :NewEnumerator0 "/Game/Animations/Characters/Templates/New_Naruto/New_Naruto_Jump_FL.New_Naruto_Jump_FL" :NewEnumerator1 "/Game/Animations/Characters/Templates/New_Naruto/New_Naruto_Jump_FL.New_Naruto_Jump_FL" :NewEnumerator2 "/Game/Animations/Characters/Templates/New_Naruto/New_Naruto_Jump_FL.New_Naruto_Jump_FL" :NewEnumerator3 "/Game/Animations/Characters/Templates/New_Naruto/New_Naruto_Jump_FL.New_Naruto_Jump_FL"))))

(fn SetFallingState
  (bind _direction (Variables|Default|GetDirection))
  (Sprite|SetFlipbook (Variables|Default|GetSprite) (select (Variables|Default|GetisFacingRight) (Utilities|Select :Index _direction :NewEnumerator0 "/Game/Animations/Characters/Templates/New_Naruto/New_Naruto_JumpFall_FR.New_Naruto_JumpFall_FR" :NewEnumerator1 "/Game/Animations/Characters/Templates/New_Naruto/New_Naruto_JumpFall_FR.New_Naruto_JumpFall_FR" :NewEnumerator2 "/Game/Animations/Characters/Templates/New_Naruto/New_Naruto_JumpFall_FR.New_Naruto_JumpFall_FR" :NewEnumerator3 "/Game/Animations/Characters/Templates/New_Naruto/New_Naruto_JumpFall_FR.New_Naruto_JumpFall_FR") (Utilities|Select :Index _direction :NewEnumerator0 "/Game/Animations/Characters/Templates/New_Naruto/New_Naruto_JumpFall_FL.New_Naruto_JumpFall_FL" :NewEnumerator1 "/Game/Animations/Characters/Templates/New_Naruto/New_Naruto_JumpFall_FL.New_Naruto_JumpFall_FL" :NewEnumerator2 "/Game/Animations/Characters/Templates/New_Naruto/New_Naruto_JumpFall_FL.New_Naruto_JumpFall_FL" :NewEnumerator3 "/Game/Animations/Characters/Templates/New_Naruto/New_Naruto_JumpFall_FL.New_Naruto_JumpFall_FL"))))

(fn SetDefendState
  (bind _direction (Variables|Default|GetDirection))
  (Sprite|SetFlipbook (Variables|Default|GetSprite) (select (Variables|Default|GetisFacingRight) (Utilities|Select :Index _direction :NewEnumerator0 "/Game/Animations/Characters/Templates/New_Naruto/New_Naruto_Defend_FR.New_Naruto_Defend_FR" :NewEnumerator1 "/Game/Animations/Characters/Templates/New_Naruto/New_Naruto_Defend_FR.New_Naruto_Defend_FR" :NewEnumerator2 "/Game/Animations/Characters/Templates/New_Naruto/New_Naruto_Defend_FR.New_Naruto_Defend_FR" :NewEnumerator3 "/Game/Animations/Characters/Templates/New_Naruto/New_Naruto_Defend_FR.New_Naruto_Defend_FR") (Utilities|Select :Index _direction :NewEnumerator0 "/Game/Animations/Characters/Templates/New_Naruto/New_Naruto_Defend_FL.New_Naruto_Defend_FL" :NewEnumerator1 "/Game/Animations/Characters/Templates/New_Naruto/New_Naruto_Defend_FL.New_Naruto_Defend_FL" :NewEnumerator2 "/Game/Animations/Characters/Templates/New_Naruto/New_Naruto_Defend_FL.New_Naruto_Defend_FL" :NewEnumerator3 "/Game/Animations/Characters/Templates/New_Naruto/New_Naruto_Defend_FL.New_Naruto_Defend_FL"))))

(fn SetAttackState)

(fn SetCrouchLandState
  (bind _direction (Variables|Default|GetDirection))
  (Sprite|SetFlipbook (Variables|Default|GetSprite) (select (Variables|Default|GetisFacingRight) (Utilities|Select :Index _direction :NewEnumerator0 "/Game/Animations/Characters/Templates/New_Naruto/New_Naruto_CrouchJump_FR.New_Naruto_CrouchJump_FR" :NewEnumerator1 "/Game/Animations/Characters/Templates/New_Naruto/New_Naruto_CrouchJump_FR.New_Naruto_CrouchJump_FR" :NewEnumerator2 "/Game/Animations/Characters/Templates/New_Naruto/New_Naruto_CrouchJump_FR.New_Naruto_CrouchJump_FR" :NewEnumerator3 "/Game/Animations/Characters/Templates/New_Naruto/New_Naruto_CrouchJump_FR.New_Naruto_CrouchJump_FR") (Utilities|Select :Index _direction :NewEnumerator0 "/Game/Animations/Characters/Templates/New_Naruto/New_Naruto_CrouchJump_FL.New_Naruto_CrouchJump_FL" :NewEnumerator1 "/Game/Animations/Characters/Templates/New_Naruto/New_Naruto_CrouchJump_FL.New_Naruto_CrouchJump_FL" :NewEnumerator2 "/Game/Animations/Characters/Templates/New_Naruto/New_Naruto_CrouchJump_FL.New_Naruto_CrouchJump_FL" :NewEnumerator3 "/Game/Animations/Characters/Templates/New_Naruto/New_Naruto_CrouchJump_FL.New_Naruto_CrouchJump_FL"))))

(fn SetCrouchJumpState
  (bind _direction (Variables|Default|GetDirection))
  (Sprite|SetFlipbook (Variables|Default|GetSprite) (select (Variables|Default|GetisFacingRight) (Utilities|Select :Index _direction :NewEnumerator0 "/Game/Animations/Characters/Templates/Naruto/Naruto_CrouchJump_FR.Naruto_CrouchJump_FR" :NewEnumerator1 "/Game/Animations/Characters/Templates/Naruto/Naruto_CrouchJump_FR.Naruto_CrouchJump_FR" :NewEnumerator2 "/Game/Animations/Characters/Templates/Naruto/Naruto_CrouchJump_FR.Naruto_CrouchJump_FR" :NewEnumerator3 "/Game/Animations/Characters/Templates/Naruto/Naruto_CrouchJump_FR.Naruto_CrouchJump_FR") (Utilities|Select :Index _direction :NewEnumerator0 "/Game/Animations/Characters/Templates/New_Naruto/New_Naruto_Walk_FL.New_Naruto_Walk_FL" :NewEnumerator1 "/Game/Animations/Characters/Templates/New_Naruto/New_Naruto_Walk_FL.New_Naruto_Walk_FL" :NewEnumerator2 "/Game/Animations/Characters/Templates/New_Naruto/New_Naruto_Walk_FL.New_Naruto_Walk_FL" :NewEnumerator3 "/Game/Animations/Characters/Templates/New_Naruto/New_Naruto_Walk_FL.New_Naruto_Walk_FL"))))

(fn SetLightAttackState
  (bind _direction (Variables|Default|GetDirection))
  (Sprite|SetFlipbook (Variables|Default|GetSprite) (select (Variables|Default|GetisFacingRight) (Utilities|Select :Index _direction :NewEnumerator0 "/Game/Animations/Characters/Templates/Naruto/Naruto_Light_Attack_FR.Naruto_Light_Attack_FR" :NewEnumerator1 "/Game/Animations/Characters/Templates/Naruto/Naruto_Light_Attack_FR.Naruto_Light_Attack_FR" :NewEnumerator2 "/Game/Animations/Characters/Templates/Naruto/Naruto_Light_Attack_FR.Naruto_Light_Attack_FR" :NewEnumerator3 "/Game/Animations/Characters/Templates/Naruto/Naruto_Light_Attack_FR.Naruto_Light_Attack_FR") (Utilities|Select :Index _direction :NewEnumerator0 "/Game/Animations/Characters/Templates/Naruto/Naruto_Defend_FL.Naruto_Defend_FL" :NewEnumerator1 "/Game/Animations/Characters/Templates/Naruto/Naruto_Defend_FL.Naruto_Defend_FL" :NewEnumerator2 "/Game/Animations/Characters/Templates/Naruto/Naruto_Defend_FL.Naruto_Defend_FL" :NewEnumerator3 "/Game/Animations/Characters/Templates/Naruto/Naruto_Defend_FL.Naruto_Defend_FL"))))

(fn SetMediumAttackState
  (bind _direction (Variables|Default|GetDirection))
  (Sprite|SetFlipbook (Variables|Default|GetSprite) (select (Variables|Default|GetisFacingRight) (Utilities|Select :Index _direction :NewEnumerator0 "/Game/Animations/Characters/Templates/Naruto/Naruto_Medium_Attack_FR.Naruto_Medium_Attack_FR" :NewEnumerator1 "/Game/Animations/Characters/Templates/Naruto/Naruto_Medium_Attack_FR.Naruto_Medium_Attack_FR" :NewEnumerator2 "/Game/Animations/Characters/Templates/Naruto/Naruto_Medium_Attack_FR.Naruto_Medium_Attack_FR" :NewEnumerator3 "/Game/Animations/Characters/Templates/Naruto/Naruto_Medium_Attack_FR.Naruto_Medium_Attack_FR") (Utilities|Select :Index _direction :NewEnumerator0 "/Game/Animations/Characters/Templates/Naruto/Naruto_Defend_FL.Naruto_Defend_FL" :NewEnumerator1 "/Game/Animations/Characters/Templates/Naruto/Naruto_Defend_FL.Naruto_Defend_FL" :NewEnumerator2 "/Game/Animations/Characters/Templates/Naruto/Naruto_Defend_FL.Naruto_Defend_FL" :NewEnumerator3 "/Game/Animations/Characters/Templates/Naruto/Naruto_Defend_FL.Naruto_Defend_FL"))))

(fn SetHeavyAttackState
  (bind _direction (Variables|Default|GetDirection))
  (Sprite|SetFlipbook (Variables|Default|GetSprite) (select (Variables|Default|GetisFacingRight) (Utilities|Select :Index _direction :NewEnumerator0 "/Game/Animations/Characters/Templates/Naruto/Naruto_Heavy_Attack_FR.Naruto_Heavy_Attack_FR" :NewEnumerator1 "/Game/Animations/Characters/Templates/Naruto/Naruto_Heavy_Attack_FR.Naruto_Heavy_Attack_FR" :NewEnumerator2 "/Game/Animations/Characters/Templates/Naruto/Naruto_Heavy_Attack_FR.Naruto_Heavy_Attack_FR" :NewEnumerator3 "/Game/Animations/Characters/Templates/Naruto/Naruto_Heavy_Attack_FR.Naruto_Heavy_Attack_FR") (Utilities|Select :Index _direction :NewEnumerator0 "/Game/Animations/Characters/Templates/Naruto/Naruto_Defend_FL.Naruto_Defend_FL" :NewEnumerator1 "/Game/Animations/Characters/Templates/Naruto/Naruto_Defend_FL.Naruto_Defend_FL" :NewEnumerator2 "/Game/Animations/Characters/Templates/Naruto/Naruto_Defend_FL.Naruto_Defend_FL" :NewEnumerator3 "/Game/Animations/Characters/Templates/Naruto/Naruto_Defend_FL.Naruto_Defend_FL"))))

(fn SetGetHurtState
  (bind _direction (Variables|Default|GetDirection))
  (Sprite|SetFlipbook (Variables|Default|GetSprite) (select (Variables|Default|GetisFacingRight) (Utilities|Select :Index _direction :NewEnumerator0 "/Game/Animations/Characters/Templates/New_Naruto/New_Naruto_GetHurt_FR.New_Naruto_GetHurt_FR" :NewEnumerator1 "/Game/Animations/Characters/Templates/New_Naruto/New_Naruto_GetHurt_FR.New_Naruto_GetHurt_FR" :NewEnumerator2 "/Game/Animations/Characters/Templates/New_Naruto/New_Naruto_GetHurt_FR.New_Naruto_GetHurt_FR" :NewEnumerator3 "/Game/Animations/Characters/Templates/New_Naruto/New_Naruto_GetHurt_FR.New_Naruto_GetHurt_FR") (Utilities|Select :Index _direction :NewEnumerator0 "/Game/Animations/Characters/Templates/New_Naruto/New_Naruto_GetHurt_FL.New_Naruto_GetHurt_FL" :NewEnumerator1 "/Game/Animations/Characters/Templates/New_Naruto/New_Naruto_GetHurt_FL.New_Naruto_GetHurt_FL" :NewEnumerator2 "/Game/Animations/Characters/Templates/New_Naruto/New_Naruto_GetHurt_FL.New_Naruto_GetHurt_FL" :NewEnumerator3 "/Game/Animations/Characters/Templates/New_Naruto/New_Naruto_GetHurt_FL.New_Naruto_GetHurt_FL"))))

(fn SetDashing/RollingState
  (bind _direction (Variables|Default|GetDirection))
  (Sprite|SetFlipbook (Variables|Default|GetSprite) (select (Variables|Default|GetisFacingRight) (Utilities|Select :Index _direction :NewEnumerator0 "/Game/Animations/Characters/Templates/New_Naruto/New_Naruto_Roll_FR.New_Naruto_Roll_FR" :NewEnumerator1 "/Game/Animations/Characters/Templates/New_Naruto/New_Naruto_Roll_FR.New_Naruto_Roll_FR" :NewEnumerator2 "/Game/Animations/Characters/Templates/New_Naruto/New_Naruto_Roll_FR.New_Naruto_Roll_FR" :NewEnumerator3 "/Game/Animations/Characters/Templates/New_Naruto/New_Naruto_Roll_FR.New_Naruto_Roll_FR") (Utilities|Select :Index _direction :NewEnumerator0 "/Game/Animations/Characters/Templates/New_Naruto/New_Naruto_Roll_FL.New_Naruto_Roll_FL" :NewEnumerator1 "/Game/Animations/Characters/Templates/New_Naruto/New_Naruto_Roll_FL.New_Naruto_Roll_FL" :NewEnumerator2 "/Game/Animations/Characters/Templates/New_Naruto/New_Naruto_Roll_FL.New_Naruto_Roll_FL" :NewEnumerator3 "/Game/Animations/Characters/Templates/New_Naruto/New_Naruto_Roll_FL.New_Naruto_Roll_FL"))))