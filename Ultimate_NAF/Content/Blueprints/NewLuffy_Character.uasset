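; Player-controlled 2D flipbook character (Luffy) that walks, runs, jumps and defends on two movement axes.
; Input events set CharacterState and movement speed, while Tick resolves movement, falling and facing, then calls per-state functions that swap left/right flipbooks.
; Most flipbooks are Rock Lee or Naruto assets, with only right-facing idle using Luffy.
; Attacking is an empty stub, and SetDirectionOld and CalculateZ are unused.
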(event Custom|DirectionAndMovementStates
  ;[1 1 1] Set Direction and Movements States
  (if (Utilities|IsFalling)
    ;;[1 1 1] If Character Is Jumping, (Even Though Character Is Falling), Don't Play Fall Anim Until Playing Is No Longer Jumping
    (if (not (Utilities|Enum|Equal(Enum) (Variables|Default|GetCharacterState) "NewEnumerator3"))
      (Variables|Default|SetCharacterState "NewEnumerator4")
      (CallFunction|SetFallingState))
    (else
      (if (and (> (Variables|/Script/Engine.CharacterMovementComponent|GetMaxWalkSpeed (Variables|Character|GetCharacterMovement)) 2e+02) (not (Utilities|IsVelocityZero)))
        (Variables|Default|SetCharacterState "NewEnumerator1"))
      (if (or (!= (Input|AxisValues|GetXAxis) 0.0) (!= (Input|AxisValues|GetYAxis) 0.0))
        (CallFunction|SetDirection :!label _label)
        (if (Utilities|Enum|Equal(Enum) (Variables|Default|GetCharacterState) "NewEnumerator0")
          (CallFunction|SetWalkingState)
          (elif (Utilities|Enum|Equal(Enum) (Variables|Default|GetCharacterState) "NewEnumerator1")
            (CallFunction|SetRunningState)))
        (else
          (Utilities|FlowControl|Delay 0.15)
          (if (or (!= (Input|AxisValues|GetXAxis) 0.0) (!= (Input|AxisValues|GetYAxis) 0.0))
            (goto _label)
            (else
              ;;[1 1 1] Check If Player Is Defending = If Not True Return To Idle
              (if (Utilities|Enum|Equal(Enum) (Variables|Default|GetCharacterState) "NewEnumerator8")
                (CallFunction|SetDefendState)
                (elif (not (Utilities|IsFalling))
                  (CallFunction|SetIdleState))))))))))

(event EventTick
  (params (DeltaSeconds :type Float%20%28single-precision%29))
  ;[1 1 1] Player Direction
  (CallFunction|DirectionandMovementStates))

(event Input|ActionEvents|InputActionDefending
  (params (Key :type Key%20Structure))
  ;[1 1 1] Defending
  (:Pressed
    (Variables|Default|SetCharacterState "NewEnumerator8")
    (CallFunction|SetDefendState))
  (:Released
    (Variables|Default|SetCharacterState "NewEnumerator6")
    (CallFunction|SetIdleState)))

(event Input|ActionEvents|InputActionJumping
  (params (Key :type Key%20Structure))
  ;[1 1 1] Jumping
  (:Pressed
    (Character|Jump)
    (Variables|Default|SetCharacterState "NewEnumerator3")
    (CallFunction|SetJumpingState)
    (Utilities|FlowControl|Delay 0.2)
    (Variables|Default|SetCharacterState "NewEnumerator4")
    (CallFunction|SetFallingState))
  (:Released
    (Character|StopJumping)))

(event Input|ActionEvents|InputActionAttacking
  (params (Key :type Key%20Structure))
  ;[1 1 1] Attacking
)

(event Input|AxisEvents|InputAxisXAxis
  (params (AxisValue :type Float%20%28single-precision%29))
  ;[1 1 1] Left and Right Movement
  (if (Math|Boolean|ORBoolean (Utilities|IsFalling) (Utilities|Enum|Equal(Enum) (Variables|Default|GetCharacterState) "NewEnumerator1") (Utilities|Enum|Equal(Enum) (Variables|Default|GetCharacterState) "NewEnumerator3") (Utilities|IsVelocityZero))
    _
    (else
      (Variables|Default|SetCharacterState "NewEnumerator0")))
  (Pawn|Input|AddMovementInput "0,1.000000, 0" AxisValue false))

(event Input|AxisEvents|InputAxisYAxis
  (params (AxisValue :type Float%20%28single-precision%29))
  ;[1 1 1] Left and Right Movement
  (if (Math|Boolean|ORBoolean (Utilities|IsFalling) (Utilities|Enum|Equal(Enum) (Variables|Default|GetCharacterState) "NewEnumerator1") (Utilities|Enum|Equal(Enum) (Variables|Default|GetCharacterState) "NewEnumerator3") (Utilities|IsVelocityZero))
    _
    (else
      (Variables|Default|SetCharacterState "NewEnumerator0")))
  (Pawn|Input|AddMovementInput "-1.000000,0.000000, 0" AxisValue false))

(event Input|KeyboardEvents|LeftShift
  (params (Key :type Key%20Structure))
  ;[1 1 1] Running
  (:Pressed
    (if (Utilities|IsVelocityGreaterThanZero)
      (Variables|Default|SetCharacterState "NewEnumerator1")
      (Variables|/Script/Engine.CharacterMovementComponent|SetMaxWalkSpeed (Variables|Character|GetCharacterMovement) 7.5e+02)
      (Development|PrintString "He is running")))
  (:Released
    (if (Utilities|IsVelocityGreaterThanZero)
      (Variables|Default|SetCharacterState "NewEnumerator0")
      (else
        (Variables|Default|SetCharacterState "NewEnumerator6")))
    (Variables|/Script/Engine.CharacterMovementComponent|SetMaxWalkSpeed (Variables|Character|GetCharacterMovement) 1.5e+02)
    (Development|PrintString "He is no longer running")))

(fn ConstructionScript
  (Transformation|SetWorldRotation (Variables|Default|GetSprite) (Math|Rotator|MakeRotator (.pitch (Transformation|GetWorldRotation (Variables|Default|GetSpringArm))) 0.0 -9e+01) false false))

(fn SetDirectionOld
  (if (or (!= (Input|AxisValues|GetXAxis) 0.0) (!= (Input|AxisValues|GetYAxis) 0.0))
    (bind _output_get (Variables|Default|SetDirection (select (> (Input|AxisValues|GetYAxis) 0.0) "NewEnumerator0" (select (< (Input|AxisValues|GetYAxis) 0.0) "NewEnumerator1" (select (> (Input|AxisValues|GetXAxis) 0.0) "NewEnumerator2" "NewEnumerator3")))))
    (switch Utilities|FlowControl|Switch|SwitchonSetDir _output_get
      (:NewEnumerator0
        _)
      (:NewEnumerator1
        _)
      (:NewEnumerator2
        (Variables|Default|SetisFacingLeft true)
        (Variables|Default|SetisFacingRight false))
      (:NewEnumerator3
        (Variables|Default|SetisFacingRight true)
        (Variables|Default|SetisFacingLeft false)))
    (return)))

(fn CalculateZ
  (bind _returnvalue (Transformation|GetActorLocation))
  (bind _returnvalue_2 (Transformation|GetActorLocation))
  (bind _outhit (Collision|LineTraceByChannel (Transformation|GetActorLocation) (Math|Vector|MakeVector (.x _returnvalue_2) (.y _returnvalue_2) (- (.z _returnvalue_2) 2e+02)) "TraceTypeQuery1" false 0 "None"))
  (Transformation|SetActorLocation (Math|Vector|MakeVector (.x _returnvalue) (.y _returnvalue) (+ (.z (.ImpactPoint (Collision|BreakHitResult _outhit))) (Variables|Default|GetDistanceZ))) false false))

(fn SetIdleState
  (bind _direction (Variables|Default|GetDirection))
  (bind _direction_2 (Variables|Default|GetDirection))
  (Variables|Default|SetCharacterState "NewEnumerator6")
  (Sprite|SetFlipbook (Variables|Default|GetSprite) (select (Utilities|IsVelocityGreaterThanZero) (select (Variables|Default|GetisFacingRight) (Utilities|Select :Index _direction_2 :NewEnumerator0 "/Game/Animations/Characters/Templates/Naruto/Naruto_Walk_FR.Naruto_Walk_FR" :NewEnumerator1 "/Game/Animations/Characters/Templates/Naruto/Naruto_Walk_FR.Naruto_Walk_FR" :NewEnumerator2 "/Game/Animations/Characters/Templates/Naruto/Naruto_Walk_FR.Naruto_Walk_FR" :NewEnumerator3 "/Game/Animations/Characters/Templates/Naruto/Naruto_Walk_FR.Naruto_Walk_FR") (Utilities|Select :Index _direction_2 :NewEnumerator0 "/Game/Animations/Characters/Templates/Naruto/Naruto_Walk_FL.Naruto_Walk_FL" :NewEnumerator1 "/Game/Animations/Characters/Templates/Naruto/Naruto_Walk_FL.Naruto_Walk_FL" :NewEnumerator2 "/Game/Animations/Characters/Templates/Naruto/Naruto_Walk_FL.Naruto_Walk_FL" :NewEnumerator3 "/Game/Animations/Characters/Templates/Naruto/Naruto_Walk_FL.Naruto_Walk_FL")) (select (Variables|Default|GetisFacingRight) (Utilities|Select :Index _direction :NewEnumerator0 "/Game/Sprites/Characters/Templates/Luffy/New_Luffy_Idle_FR.New_Luffy_Idle_FR" :NewEnumerator1 "/Game/Sprites/Characters/Templates/Luffy/New_Luffy_Idle_FR.New_Luffy_Idle_FR" :NewEnumerator2 "/Game/Sprites/Characters/Templates/Luffy/New_Luffy_Idle_FR.New_Luffy_Idle_FR" :NewEnumerator3 "/Game/Sprites/Characters/Templates/Luffy/New_Luffy_Idle_FR.New_Luffy_Idle_FR") (Utilities|Select :Index _direction :NewEnumerator0 "/Game/Animations/Characters/Templates/Rock_Lee/RockLee_Idle_FL.RockLee_Idle_FL" :NewEnumerator1 "/Game/Animations/Characters/Templates/Rock_Lee/RockLee_Idle_FL.RockLee_Idle_FL" :NewEnumerator2 "/Game/Animations/Characters/Templates/Rock_Lee/RockLee_Idle_FL.RockLee_Idle_FL" :NewEnumerator3 "/Game/Animations/Characters/Templates/Rock_Lee/RockLee_Idle_FL.RockLee_Idle_FL")))))

(fn SetDirection
  (bind _output_get (Variables|Default|SetDirection (select (> (Input|AxisValues|GetYAxis) 0.0) "NewEnumerator0" (select (< (Input|AxisValues|GetYAxis) 0.0) "NewEnumerator1" (select (> (Input|AxisValues|GetXAxis) 0.0) "NewEnumerator2" "NewEnumerator3")))))
  (switch Utilities|FlowControl|Switch|SwitchonSetDir _output_get
    (:NewEnumerator0
      _)
    (:NewEnumerator1
      _)
    (:NewEnumerator2
      (Variables|Default|SetisFacingLeft true)
      (Variables|Default|SetisFacingRight false))
    (:NewEnumerator3
      (Variables|Default|SetisFacingRight true)
      (Variables|Default|SetisFacingLeft false)))
  (return))

(fn SetWalkingState
  (bind _direction (Variables|Default|GetDirection))
  (Sprite|SetFlipbook (Variables|Default|GetSprite) (select (Variables|Default|GetisFacingRight) (Utilities|Select :Index _direction :NewEnumerator0 "/Game/Animations/Characters/Templates/Rock_Lee/RockLee_Walk_FR.RockLee_Walk_FR" :NewEnumerator1 "/Game/Animations/Characters/Templates/Rock_Lee/RockLee_Walk_FR.RockLee_Walk_FR" :NewEnumerator2 "/Game/Animations/Characters/Templates/Rock_Lee/RockLee_Walk_FR.RockLee_Walk_FR" :NewEnumerator3 "/Game/Animations/Characters/Templates/Rock_Lee/RockLee_Walk_FR.RockLee_Walk_FR") (Utilities|Select :Index _direction :NewEnumerator0 "/Game/Animations/Characters/Templates/Rock_Lee/RockLee_Walk_FL.RockLee_Walk_FL" :NewEnumerator1 "/Game/Animations/Characters/Templates/Rock_Lee/RockLee_Walk_FL.RockLee_Walk_FL" :NewEnumerator2 "/Game/Animations/Characters/Templates/Rock_Lee/RockLee_Walk_FL.RockLee_Walk_FL" :NewEnumerator3 "/Game/Animations/Characters/Templates/Rock_Lee/RockLee_Walk_FL.RockLee_Walk_FL"))))

(fn SetRunningState
  (Sprite|SetFlipbook (Variables|Default|GetSprite) (select (Variables|Default|GetisFacingRight) (Utilities|Select :Index (Variables|Default|GetDirection) :NewEnumerator0 "/Game/Animations/Characters/Templates/Rock_Lee/RockLee_Run_FR.RockLee_Run_FR" :NewEnumerator1 "/Game/Animations/Characters/Templates/Rock_Lee/RockLee_Run_FR.RockLee_Run_FR" :NewEnumerator2 "/Game/Animations/Characters/Templates/Rock_Lee/RockLee_Run_FR.RockLee_Run_FR" :NewEnumerator3 "/Game/Animations/Characters/Templates/Rock_Lee/RockLee_Run_FR.RockLee_Run_FR") (Utilities|Select :Index (Variables|Default|GetDirection) :NewEnumerator0 "/Game/Animations/Characters/Templates/Rock_Lee/RockLee_Run_FL.RockLee_Run_FL" :NewEnumerator1 "/Game/Animations/Characters/Templates/Rock_Lee/RockLee_Run_FL.RockLee_Run_FL" :NewEnumerator2 "/Game/Animations/Characters/Templates/Rock_Lee/RockLee_Run_FL.RockLee_Run_FL" :NewEnumerator3 "/Game/Animations/Characters/Templates/Rock_Lee/RockLee_Run_FL.RockLee_Run_FL"))))

(fn SetJumpingState
  (bind _direction (Variables|Default|GetDirection))
  (Sprite|SetFlipbook (Variables|Default|GetSprite) (select (Variables|Default|GetisFacingRight) (Utilities|Select :Index _direction :NewEnumerator0 "/Game/Animations/Characters/Templates/Rock_Lee/RockLee_Jump_FR.RockLee_Jump_FR" :NewEnumerator1 "/Game/Animations/Characters/Templates/Rock_Lee/RockLee_Jump_FR.RockLee_Jump_FR" :NewEnumerator2 "/Game/Animations/Characters/Templates/Rock_Lee/RockLee_Jump_FR.RockLee_Jump_FR" :NewEnumerator3 "/Game/Animations/Characters/Templates/Rock_Lee/RockLee_Jump_FR.RockLee_Jump_FR") (Utilities|Select :Index _direction :NewEnumerator0 "/Game/Animations/Characters/Templates/Rock_Lee/RockLee_Jump_FL.RockLee_Jump_FL" :NewEnumerator1 "/Game/Animations/Characters/Templates/Rock_Lee/RockLee_Jump_FL.RockLee_Jump_FL" :NewEnumerator2 "/Game/Animations/Characters/Templates/Rock_Lee/RockLee_Jump_FL.RockLee_Jump_FL" :NewEnumerator3 "/Game/Animations/Characters/Templates/Rock_Lee/RockLee_Jump_FL.RockLee_Jump_FL"))))

(fn SetFallingState
  (bind _direction (Variables|Default|GetDirection))
  (Sprite|SetFlipbook (Variables|Default|GetSprite) (select (Variables|Default|GetisFacingRight) (Utilities|Select :Index _direction :NewEnumerator0 "/Game/Animations/Characters/Templates/Rock_Lee/RockLee_JumpFall_FR.RockLee_JumpFall_FR" :NewEnumerator1 "/Game/Animations/Characters/Templates/Rock_Lee/RockLee_JumpFall_FR.RockLee_JumpFall_FR" :NewEnumerator2 "/Game/Animations/Characters/Templates/Rock_Lee/RockLee_JumpFall_FR.RockLee_JumpFall_FR" :NewEnumerator3 "/Game/Animations/Characters/Templates/Rock_Lee/RockLee_JumpFall_FR.RockLee_JumpFall_FR") (Utilities|Select :Index _direction :NewEnumerator0 "/Game/Animations/Characters/Templates/Rock_Lee/RockLee_JumpFall_FL.RockLee_JumpFall_FL" :NewEnumerator1 "/Game/Animations/Characters/Templates/Rock_Lee/RockLee_JumpFall_FL.RockLee_JumpFall_FL" :NewEnumerator2 "/Game/Animations/Characters/Templates/Rock_Lee/RockLee_JumpFall_FL.RockLee_JumpFall_FL" :NewEnumerator3 "/Game/Animations/Characters/Templates/Rock_Lee/RockLee_JumpFall_FL.RockLee_JumpFall_FL"))))

(fn SetDefendState
  (bind _direction (Variables|Default|GetDirection))
  (Sprite|SetFlipbook (Variables|Default|GetSprite) (select (Variables|Default|GetisFacingRight) (Utilities|Select :Index _direction :NewEnumerator0 "/Game/Animations/Characters/Templates/Rock_Lee/RockLee_Defend_FR.RockLee_Defend_FR" :NewEnumerator1 "/Game/Animations/Characters/Templates/Rock_Lee/RockLee_Defend_FR.RockLee_Defend_FR" :NewEnumerator2 "/Game/Animations/Characters/Templates/Rock_Lee/RockLee_Defend_FR.RockLee_Defend_FR" :NewEnumerator3 "/Game/Animations/Characters/Templates/Rock_Lee/RockLee_Defend_FR.RockLee_Defend_FR") (Utilities|Select :Index _direction :NewEnumerator0 "/Game/Animations/Characters/Templates/Rock_Lee/RockLee_Defend_FL.RockLee_Defend_FL" :NewEnumerator1 "/Game/Animations/Characters/Templates/Rock_Lee/RockLee_Defend_FL.RockLee_Defend_FL" :NewEnumerator2 "/Game/Animations/Characters/Templates/Rock_Lee/RockLee_Defend_FL.RockLee_Defend_FL" :NewEnumerator3 "/Game/Animations/Characters/Templates/Rock_Lee/RockLee_Defend_FL.RockLee_Defend_FL"))))

(fn SetAttackState)